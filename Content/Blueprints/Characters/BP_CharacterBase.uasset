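; BP_CharacterBase is a base character Blueprint that uses the Gameplay Ability System for melee combat and handles death.
; It acquires GA_Melee on BeginPlay and activates it through the ability system component on MeleeAttack.
; Sword collider overlaps with other hostile characters send a damage gameplay event to itself, with the victim as payload target.
; Die plays a death montage, waits its duration, then destroys the actor.
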(event `self.ReceiveBeginPlay`
  (`self.AquireAbility` "/Game/Blueprints/Characters/GameplayAbilities/Melee/GA_Melee.GA_Melee_C"))

(event `MeleeAttack`
  (`AbilitySystemComponent.TryActivateAbilityByClass` (`self.AbilitySystemComp`) "/Game/Blueprints/Characters/GameplayAbilities/Melee/GA_Melee.GA_Melee_C" true))

(event `self.SwordCollider.OnComponentBeginOverlap`
  (params (OverlappedComponent :type "PrimitiveComponent Object Reference") (OtherActor :type "Actor Object Reference") (OtherComp :type "PrimitiveComponent Object Reference") (OtherBodyIndex :type Integer) (bFromSweep :type Boolean) (SweepResult :type "HitResult Structure (by ref)"))
  (bind _asbp_character_base (cast `/Game/Blueprints/Characters/BP_CharacterBase` OtherActor))
  (bind _returnvalue (`self.IsOtherHostile` _asbp_character_base self))
  (if (and (!= OtherActor self) _returnvalue)
    (`AbilitySystemBlueprintLibrary.SendGameplayEventToActor` self (struct :`TagName` "skill.melee.dealDamage") (make `GameplayEventData` (struct) null OtherActor))))

(event `self.BP_Die`
  (bind _returnvalue (`self.PlayAnimMontage` "/Game/Blueprints/Characters/Animation/AM_Die_Shinbi.AM_Die_Shinbi"))
  (`KismetSystemLibrary.Delay` _returnvalue)
  (`self.K2_DestroyActor`))

(fn `UserConstructionScript`)